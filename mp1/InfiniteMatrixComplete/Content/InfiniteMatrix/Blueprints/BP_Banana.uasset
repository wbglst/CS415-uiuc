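; BP_Banana is a health pickup that restores 50 health, capped at 100, when BP_Player overlaps its mesh, with a pop sound.
; Player overlap with either the mesh or Triggerzone asks BananaSpawner for another healthpack and destroys the banana; Triggerzone grants no health.
; Randomexist, uncalled here, destroys the actor unless a random float exactly equals 7, so almost always.
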(event OnComponentBeginOverlap(StaticMesh)
  (params (OverlappedComponent :type Primitive%20Component%20Object%20Reference) (OtherActor :type Actor%20Object%20Reference) (OtherComp :type Primitive%20Component%20Object%20Reference) (OtherBodyIndex :type Integer) (bFromSweep :type Boolean) (SweepResult :type Hit%20Result%20Structure%20%28by%20ref%29))
  (bind _asbp_player (Utilities|Casting|CastToBP_Player OtherActor))
  (Audio|PlaySoundatLocation "/Game/InfiniteMatrix/audio/S_Pop.S_Pop" (Transformation|GetActorLocation) "0, 0, 0" 1.0 1.0 0.0 0 0 0 0)
  (Variables|/Game/InfiniteMatrix/Blueprints/BP_Player.BP_Player_C|Sethealth _asbp_player (Math|Float|Min(Float) (+ (Variables|/Game/InfiniteMatrix/Blueprints/BP_Player.BP_Player_C|Gethealth _asbp_player) 5e+01) 1e+02))
  (Default|SpawnHealthpackatSpawn (Variables|Default|GetBananaSpawner))
  (Actor|DestroyActor))

(event OnComponentBeginOverlap(triggerzone)
  (params (OverlappedComponent :type Primitive%20Component%20Object%20Reference) (OtherActor :type Actor%20Object%20Reference) (OtherComp :type Primitive%20Component%20Object%20Reference) (OtherBodyIndex :type Integer) (bFromSweep :type Boolean) (SweepResult :type Hit%20Result%20Structure%20%28by%20ref%29))
  (Utilities|Casting|CastToBP_Player OtherActor)
  (Default|SpawnHealthpackatSpawn (Variables|Default|GetBananaSpawner))
  (Actor|DestroyActor))

(event EventTick
  (params (DeltaSeconds :type Float%20%28single-precision%29)))

(fn ConstructionScript)

(fn Randomexist
  (if (not (== (Math|Random|RandomFloatinRange 1e+01 0.0) 7.0))
    (Actor|DestroyActor)))