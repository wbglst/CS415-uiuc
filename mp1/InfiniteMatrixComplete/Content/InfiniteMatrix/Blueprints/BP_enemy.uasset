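; BP_enemy is an enemy actor that damages the player on contact and awards score when shot.
; Its StaticMesh overlap either lowers BP_Player health, showing restart at zero, or credits the bullet's owning player and destroys the bullet.
; A separate Passenemy overlap removes the enemy without damage or score when the player touches it.
; Every handled hit asks Enemyspawner for a replacement before the enemy destroys itself.
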(event OnComponentBeginOverlap(StaticMesh)
  (params (OverlappedComponent :type Primitive%20Component%20Object%20Reference) (OtherActor :type Actor%20Object%20Reference) (OtherComp :type Primitive%20Component%20Object%20Reference) (OtherBodyIndex :type Integer) (bFromSweep :type Boolean) (SweepResult :type Hit%20Result%20Structure%20%28by%20ref%29))
  (bind _asbp_player (Utilities|Casting|CastToBP_Player OtherActor)
    (:then
      (bind _output_get (Variables|/Game/InfiniteMatrix/Blueprints/BP_Player.BP_Player_C|Sethealth _asbp_player (Math|Float|Max(Float) (- (Variables|/Game/InfiniteMatrix/Blueprints/BP_Player.BP_Player_C|Gethealth _asbp_player) 1e+01) 0.0)))
      (Default|SpawnEnemyatSpawn (Variables|Default|Getenemyspawner))
      (Actor|DestroyActor)
      (bind _output_get_2 (Variables|/Game/InfiniteMatrix/Blueprints/BP_Player.BP_Player_C|SetIsDead _asbp_player (== _output_get 0.0)))
      (if _output_get_2
        (Default|DisplayRestart _asbp_player)))
    (:CastFailed
      (bind _asbp_bullet (Utilities|Casting|CastToBP_Bullet OtherActor))
      (Variables|/Game/InfiniteMatrix/Blueprints/BP_Player.BP_Player_C|SetScore (Variables|/Game/InfiniteMatrix/Blueprints/BP_Bullet.BP_Bullet_C|Getcurrplayer _asbp_bullet) (+ (Variables|/Game/InfiniteMatrix/Blueprints/BP_Player.BP_Player_C|GetScore (Variables|/Game/InfiniteMatrix/Blueprints/BP_Bullet.BP_Bullet_C|Getcurrplayer _asbp_bullet)) 1.0))
      (Default|SpawnEnemyatSpawn (Variables|Default|Getenemyspawner))
      (Actor|DestroyActor _asbp_bullet)
      (Actor|DestroyActor))))

(event OnComponentBeginOverlap(passenemy)
  (params (OverlappedComponent :type Primitive%20Component%20Object%20Reference) (OtherActor :type Actor%20Object%20Reference) (OtherComp :type Primitive%20Component%20Object%20Reference) (OtherBodyIndex :type Integer) (bFromSweep :type Boolean) (SweepResult :type Hit%20Result%20Structure%20%28by%20ref%29))
  (Utilities|Casting|CastToBP_Player OtherActor)
  (Default|SpawnEnemyatSpawn (Variables|Default|Getenemyspawner))
  (Actor|DestroyActor))

(event EventBeginPlay)

(event Collision|EventActorBeginOverlap
  (params (OtherActor :type Actor%20Object%20Reference)))

(event EventTick
  (params (DeltaSeconds :type Float%20%28single-precision%29)))

(fn ConstructionScript)